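; Player actor that plays a looping idle animation on its Sphere and Donut components, plus a sinking death move.
; A looping timer set on BeginPlay fires MoveDonut, which updates MovingDistance and eases the Sphere vertically while rotating the Donut through MoveComponentTo.
; DeathMove zeroes the idle distance and rotation instead of clearing the timer, then eases the Sphere downward.
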(event `self.ReceiveBeginPlay`
  (`KismetSystemLibrary.K2_SetTimerDelegate` (delegate `MoveDonut`) (+ (`self.WaitTimeBeforeChange`) (`self.MovingTime`)) true))

(event `MoveDonut`
  (bind _moving_distance (`self.Moving Distance`))
  (`|ExecutionSequence`
    (:`then_0`
      (bind _result (`/Engine/EditorBlueprintResources/StandardMacros.NegateFloat` _moving_distance)
        (:`  `
          (set `self.Moving Distance` _result)
          (`KismetSystemLibrary.MoveComponentTo` (`self.Sphere`) (* (`KismetMathLibrary.Vector_Up`) _moving_distance) (struct) true true (`self.MovingTime`)))))
    (:`then_1`
      (bind _result_2 (`/Engine/EditorBlueprintResources/StandardMacros.NegateFloat` (`self.Donut_Ref`))
        (:`  `
          (`KismetSystemLibrary.MoveComponentTo` (`self.Donut`) (0.0 0.0 0.0) (* (`self.DonutRotation`) _result_2) true true (`self.MovingTime`)))))))

(event `DeathMove`
  ;[1 1 1] Death Movement
  (set `self.Moving Distance` 0.0)
  (set `self.DonutRotation` (struct))
  (`KismetSystemLibrary.MoveComponentTo` (`self.Sphere`) (0.0 0.0 -400.0) (struct) true true 1.5))

(fn `UserConstructionScript`)