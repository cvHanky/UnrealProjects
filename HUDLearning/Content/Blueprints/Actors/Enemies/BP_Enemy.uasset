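; BP_Enemy is an enemy actor that takes damage, can die, and can strike back at the player.
; Incoming damage is reduced by Armor and capped at Health, with separate sounds for a block, a hit and death.
; A surviving enemy with WillRetaliate set calls AttackPlayer, which applies Attack plus optional bonus damage to the first player controller rather than its pawn.
; Death only sets the IsDead flag, which blocks further damage.
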(event `self.ReceiveAnyDamage`
  (params (Damage :type "Float (single-precision)") (DamageType :type "DamageType Object Reference") (InstigatedBy :type "Controller Object Reference") (DamageCauser :type "Actor Object Reference"))
  (bind _health (`self.Health`))
  (bind _returnvalue (`KismetMathLibrary.FClamp` (- Damage (`self.Armor`)) 0.0 _health))
  ;[1 1 1] Taking Damage
  (if (not (`self.IsDead`))
    (if (== _returnvalue 0.0)
      ;;[1 1 1] Play "blocking" sound
      (`GameplayStatics.PlaySound2D` "/Engine/VREditor/Sounds/UI/Click_on_Button.Click_on_Button" 1.0 1.0 0.0 null null)
      (else
        (bind _output_get (set `self.Health` (- _health _returnvalue)))
        (if (<= _output_get 0.0)
          (set `self.IsDead` true)
          (`GameplayStatics.PlaySound2D` "/Engine/EditorSounds/GamePreview/PossessPlayer.PossessPlayer" 1.0 1.0 0.0 null null)
          (else
            (`GameplayStatics.PlaySound2D` "/Engine/VREditor/Sounds/UI/Object_PickUp.Object_PickUp" 1.0 1.0 0.0 null null)
            (if (`self.WillRetaliate`)
              (`self.AttackPlayer` 0.0))))))))

(event `AttackPlayer`
  (params (AdditionalDMG :type "Float (double-precision)"))
  ;[1 1 1] Attacking the player
  (`GameplayStatics.ApplyDamage` (`GameplayStatics.GetPlayerController` 0) (+ AdditionalDMG (`self.Attack`))))

(fn `UserConstructionScript`)