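; Player controller for a card-based combat game that holds player combat state and manages the current enemy.
; Incoming damage is reduced by Defense and subtracted from Health with sound feedback; reaching zero marks death and triggers DeathMove on the player pawn.
; DamageCard applies card damage plus Attack to CurrentEnemy.
; SpawnEnemy places one enemy at the BP_EnemySpawn actor and stores it as CurrentEnemy, guarded by IsEnemyPresent.
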(event `self.ReceiveAnyDamage`
  (params (Damage :type "Float (single-precision)") (DamageType :type "DamageType Object Reference") (InstigatedBy :type "Controller Object Reference") (DamageCauser :type "Actor Object Reference"))
  (bind _returnvalue (- Damage (`self.Defense`)))
  ;[1 1 1] Player Takes Damage
  (if (<= _returnvalue 0.0)
    (`GameplayStatics.PlaySound2D` "/Engine/VREditor/Sounds/UI/Drop_Item_From_ContentBrowser.Drop_Item_From_ContentBrowser" 1.0 1.0 0.0 null null)
    (elif (not (`self.IsDead`))
      (bind _output_get (set `self.Health` (`KismetMathLibrary.FClamp` (- (`self.Health`) (`KismetMathLibrary.FClamp` _returnvalue 0.0 (`self.MaxHealth`))) 0.0 (`self.MaxHealth`))))
      (if (<= _output_get 0.0)
        ;[1 1 1] Player Death
        (set `self.IsDead` true)
        (`GameplayStatics.PlaySound2D` "/Game/StarterContent/Audio/Collapse02.Collapse02" 1.0 1.0 0.0 null null)
        (bind _asplayer_blueprint (cast `/Game/Blueprints/Actors/Player_Blueprint` (`GameplayStatics.GetPlayerPawn` 0)))
        (`/Game/Blueprints/Actors/Player_Blueprint.DeathMove` _asplayer_blueprint)
        (else
          (`GameplayStatics.PlaySound2D` "/Engine/VREditor/Sounds/UI/Camera_Shutter.Camera_Shutter" 1.0 1.0 0.0 null null))))))

(event `DamageCard`
  (params (Damage :type "Float (double-precision)"))
  (`GameplayStatics.ApplyDamage` (`self.CurrentEnemy`) (+ Damage (`self.Attack`)) self))

(event `SpawnEnemy`
  (params (Enemy :type "/Game/Blueprints/Actors/Enemy_Blueprint Class Reference"))
  ;[1 1 1] Spawn Enemy
  (if (not (`self.IsEnemyPresent`))
    (bind _returnvalue (`GameplayStatics.GetActorOfClass` "/Game/Blueprints/Actors/BP_EnemySpawn.BP_EnemySpawn_C"))
    (bind _returnvalue_2 (`|SpawnActorFromClass` Enemy (`self.GetTransform` _returnvalue) "Undefined" "MultiplyWithRoot" null null))
    (set `self.IsEnemyPresent` true)
    (set `self.CurrentEnemy` _returnvalue_2)))

(fn `UserConstructionScript`)