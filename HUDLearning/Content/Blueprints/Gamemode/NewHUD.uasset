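; NewHUD is a HUD Blueprint that toggles the screen between a fight UI and a map view.
; Its Construction Script creates the WB_UI and WB_Map widgets, stores references and adds both to the viewport, with only the map visible.
; BeginPlay switches to the fight UI.
; The MapSwitch and FightSwitch events call functions that show one widget and hide the other, without recreating either.
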(event `self.ReceiveBeginPlay`
  (`self.Switch to Fight`))

(event `MapSwitch`
  (`self.SwitchToMap`))

(event `FightSwitch`
  (`self.Switch to Fight`))

(fn `Switch to Fight`
  (`Widget.SetVisibility` (`self.Map_Ref`) "Hidden")
  (`Widget.SetVisibility` (`self.UI_Ref`) "Visible"))

(fn `SwitchToMap`
  (`Widget.SetVisibility` (`self.UI_Ref`) "Hidden")
  (`Widget.SetVisibility` (`self.Map_Ref`) "Visible"))

(fn `UserConstructionScript`
  (`|ExecutionSequence`
    (:`then_0`
      (bind _returnvalue (`|GenericCreateObject` "/Game/Blueprints/Gamemode/Widgets/WB_UI.WB_UI_C"))
      (bind _output_get (set `self.UI_Ref` _returnvalue))
      (`UserWidget.AddToViewport` _output_get 0)
      (set `Widget.Visibility` "Hidden" _output_get))
    (:`then_1`
      (bind _returnvalue_2 (`|GenericCreateObject` "/Game/Blueprints/Gamemode/Widgets/WB_Map.WB_Map_C"))
      (bind _output_get_2 (set `self.Map_Ref` _returnvalue_2))
      (`UserWidget.AddToViewport` _output_get_2 0)
      (set `Widget.Visibility` "Visible" _output_get_2))))