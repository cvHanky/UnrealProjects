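; Inventory component that manages a card game's collection and its in-fight deck, hand and discard piles.
; Fight start copies the Inventory into the Deck and shuffles it; fight end clears all three piles.
; Drawing moves the top card to the hand, first reshuffling the discard pile into the deck when it is empty, and returns the card data and hand index.
; Discarding moves a hand card to the discard pile.
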(fn `AddCardToInventory`
  (params (NewItem :type "PrimaryDataAsset Object Reference (by ref)"))
  (returns (OutputPin :type "PrimaryDataAsset Object Reference (by ref)"))
  (`KismetArrayLibrary.Array_Add` (`self.Inventory`) NewItem)
  (return NewItem))

(fn `DiscardCard`
  (params (HandIndex :type Integer))
  (`KismetArrayLibrary.Array_Add` (`self.Discard`) (`|GetArrayItem` (`self.Hand`) HandIndex))
  (`KismetArrayLibrary.Array_Remove` (`self.Hand`) HandIndex))

(fn `DrawCard`
  (returns (CardData :type "/Game/Blueprints/Inventory/Cards/CardLogic/DA_CardData Object Reference") (Index :type Integer))
  (locals (Card :type "/Game/Blueprints/Inventory/Cards/CardLogic/DA_CardData Object Reference") (CardIndex :type Integer))
  (bind _output (`|GetArrayItem` (`self.Deck`)))
  (bind _output_2 (`|GetArrayItem` (`self.Deck`)))
  (if (`KismetArrayLibrary.Array_IsEmpty` (`self.Deck`))
    ;[1 1 1] Deck has no cards
    (bind _issuccesful (`self.ReshuffleCards`))
    (if _issuccesful
      (bind _returnvalue (`KismetArrayLibrary.Array_Add` (`self.Hand`) _output))
      (set `local.CardIndex` _returnvalue)
      (bind _asda_card_data (cast `/Game/Blueprints/Inventory/Cards/CardLogic/DA_CardData` _output))
      (set `local.Card` _asda_card_data)
      (`KismetArrayLibrary.Array_Remove` (`self.Deck`))
      (return (`local.Card`) (`local.CardIndex`)))
    (else
      ;[1 1 1] Deck has cards
      (bind _returnvalue_2 (`KismetArrayLibrary.Array_Add` (`self.Hand`) _output_2))
      (set `local.CardIndex` _returnvalue_2)
      (bind _asda_card_data_2 (cast `/Game/Blueprints/Inventory/Cards/CardLogic/DA_CardData` _output_2))
      (set `local.Card` _asda_card_data_2)
      (`KismetArrayLibrary.Array_Remove` (`self.Deck`))
      (return (`local.Card`) (`local.CardIndex`)))))

(fn `EndOfFight`
  (`KismetArrayLibrary.Array_Clear` (`self.Deck`))
  (`KismetArrayLibrary.Array_Clear` (`self.Hand`))
  (`KismetArrayLibrary.Array_Clear` (`self.Discard`)))

(fn `ReshuffleCards`
  (returns (IsSuccesful :type Boolean))
  (locals (IsSucceded :type Boolean))
  (bind _discard (`self.Discard`))
  (if (`KismetArrayLibrary.Array_IsEmpty` _discard)
    (set `local.IsSucceded` false)
    (else
      (`KismetArrayLibrary.Array_Append` (`self.Deck`) _discard)
      (`KismetArrayLibrary.Array_Clear` (`self.Discard`))
      (`KismetArrayLibrary.Array_Shuffle` (`self.Deck`))
      (set `local.IsSucceded` true)))
  (return (`local.IsSucceded`)))

(fn `StartOfFight`
  (bind _deck (`self.Deck`))
  (`KismetArrayLibrary.Array_Append` _deck (`self.Inventory`))
  (`KismetArrayLibrary.Array_Shuffle` _deck))